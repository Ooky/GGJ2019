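; Static gravity cube that turns the player's gravity on overlap, based on the cube's orientation.
; If its up vector, compared as a string, is not world up, it calls TurnGravR for negative Y and TurnGravL otherwise on player pawn 0.
; A DoOnce gates the turn and resets shortly after overlap ends.
; The construction script applies CubeColor; an alternative position-based turn branch is left unconnected.
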(event `self.ReceiveActorBeginOverlap`
  (params (OtherActor :type "Actor Object Reference"))
  (bind _returnvalue (`GameplayStatics.GetPlayerPawn` 0))
  (bind _returnvalue_2 (`KismetStringLibrary.Conv_VectorToString` (`SceneComponent.GetUpVector` (`self.Cube`))))
  (`/Engine/EditorBlueprintResources/StandardMacros.DoOnce` false :!label _label
    (:`Completed`
      ;[1 1 1] If upvector is up, do nothing, if not:
      (if (== (`KismetStringLibrary.Conv_VectorToString` (`KismetMathLibrary.MakeVector` 0.0 0.0 1.0)) _returnvalue_2)
        _
        (elif (== (`KismetStringLibrary.Conv_VectorToString` (`KismetMathLibrary.MakeVector` 0.0 -1.0 0.0)) _returnvalue_2)
          (bind _asplayer (cast `/Game/Blueprints/Player` _returnvalue))
          (`/Game/Blueprints/Player.turnGravR` _asplayer)
          (else
            (bind _asplayer_2 (cast `/Game/Blueprints/Player` _returnvalue))
            (`/Game/Blueprints/Player.turnGravL` _asplayer_2)))))))

(event `self.ReceiveActorEndOverlap`
  (params (OtherActor :type "Actor Object Reference"))
  (`KismetSystemLibrary.Delay` 0.2)
  (goto _label :!via `Reset`))

(fn `UserConstructionScript`
  (`PrimitiveComponent.SetMaterial` (`self.Cube`) 0 (`self.CubeColor`)))