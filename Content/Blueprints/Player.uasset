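; Player rolling-ball pawn with switchable gravity for running on floor, walls and ceiling.
; Tick overwrites the ball's velocity with the Gravity vector as fake gravity and derives InAir from a Hit flag it resets each frame.
; When grounded, move inputs apply force, plus torque sideways, oriented by the current surface.
; SwitchGravity flips gravity 180°; TurnGravR/L turn it 90°, all rotating ball, camera and spring arm to match.
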(event `self.ReceiveHit`
  (params (MyComp :type "PrimitiveComponent Object Reference") (Other :type "Actor Object Reference") (OtherComp :type "PrimitiveComponent Object Reference") (bSelfMoved :type Boolean) (HitLocation :type "Vector Structure") (HitNormal :type "Vector Structure") (NormalImpulse :type "Vector Structure") (Hit :type "HitResult Structure (by ref)"))
  ;[1 1 1] InAir Check
  (bind _output_get (set `self.isHittingFloorOrWall` true)))

(event `self.ReceiveTick`
  (params (DeltaSeconds :type "Float (single-precision)"))
  ;[1 1 1] Apply Fake Gravity
  (`|ExecutionSequence`
    (:`then_0`
      ;[1 1 1] InAir Check
      (if (stale `self.ReceiveHit` _output_get)
        (set `self.inAir` false)
        (else
          (set `self.inAir` true)))
      (set `self.isHittingFloorOrWall` false))
    (:`then_1`
      (`PrimitiveComponent.SetPhysicsLinearVelocity` (`self.Ball`) (`self.Gravity`) false "None"))))

(event `InputAxis|MoveRight`
  (params (AxisValue :type "Float (single-precision)"))
  (bind _ball (`self.Ball`))
  (bind _ball_2 (`self.Ball`))
  (bind _returnvalue (* (`self.RollTorque`) (* AxisValue (* (`KismetMathLibrary.Dot_VectorVector` (`KismetMathLibrary.Normal` (`self.Gravity`)) (1.0 1.0 1.0)) -1.0)) -1.0))
  ;[1 1 1] Roll left/right
  (if (not (`self.inAir`))
    (if (`self.GravityFloorOrCeiling`)
      ;;[1 1 1] Left Right Force on Floor/Ceiling
      (`PrimitiveComponent.AddTorqueInRadians` _ball (`KismetMathLibrary.MakeVector` _returnvalue) "None" false)
      (`PrimitiveComponent.AddForce` _ball (`KismetMathLibrary.MakeVector` 0.0 (* _returnvalue -1.0)) "None" false)
      (else
        ;;[1 1 1] Left Right Force on the walls
        (`PrimitiveComponent.AddTorqueInRadians` _ball_2 (`KismetMathLibrary.MakeVector` _returnvalue) "None" false)
        (`PrimitiveComponent.AddForce` _ball_2 (`KismetMathLibrary.MakeVector` 0.0 0.0 _returnvalue) "None" false)))))

(event `InputAxis|MoveForward`
  (params (AxisValue :type "Float (single-precision)"))
  ;[1 1 1] Roll forwards/backwards
  (if (not (`self.inAir`))
    (`PrimitiveComponent.AddForce` (`self.Ball`) (`KismetMathLibrary.MakeVector` (* (`self.RollTorque`) AxisValue)) "None" false)))

(event `InputAction|SwitchGravity`
  (params (Key :type "Key Structure"))
  (bind _springarm (`self.SpringArm`))
  ;[1 1 1] Change Gravity
  ;;[1 1 1] Turn Camera and Ball
  (:`Pressed`
    (bind _output_get (set `self.Gravity` (`KismetMathLibrary.RotateAngleAxis` (`self.Gravity`) -180.0 (1.0 0.0 0.0))))
    (`SceneComponent.K2_AddLocalRotation` (`self.Camera`) (struct :`Roll` 180.0) false false)
    (`SceneComponent.K2_AddLocalRotation` (`self.Ball`) (struct :`Roll` 180.0) false false)
    ;;[1 1 1] Turn Camera Arm
    (if (`self.GravityFloorOrCeiling`)
      (`SceneComponent.K2_SetRelativeRotation` _springarm (`KismetMathLibrary.RotatorFromAxisAndAngle` (0.0 1.0 0.0) (* (`KismetMathLibrary.Dot_VectorVector` (`KismetMathLibrary.Normal` _output_get) (1.0 1.0 1.0)) -45.0)) false false)
      (else
        (`SceneComponent.K2_SetRelativeRotation` _springarm (`KismetMathLibrary.RotatorFromAxisAndAngle` (0.0 0.0 1.0) (* (`KismetMathLibrary.Dot_VectorVector` (`KismetMathLibrary.Normal` _output_get) (1.0 1.0 1.0)) 45.0)) false false)))))

(fn `turnGravL`
  (bind _springarm (`self.SpringArm`))
  ;[1 1 1] Change Gravity
  ;;[1 1 1] Turn Camera and Ball
  (bind _output_get (set `self.GravityFloorOrCeiling` (not (`self.GravityFloorOrCeiling`))))
  (bind _output_get_2 (set `self.Gravity` (`KismetMathLibrary.RotateAngleAxis` (`self.Gravity`) -90.0 (1.0 0.0 0.0))))
  (`SceneComponent.K2_AddLocalRotation` (`self.Camera`) (struct :`Roll` 90.0) false false)
  (`SceneComponent.K2_AddLocalRotation` (`self.Ball`) (struct :`Roll` 90.0) false false)
  ;;[1 1 1] Turn Camera Arm
  (if _output_get
    (`SceneComponent.K2_SetRelativeRotation` _springarm (`KismetMathLibrary.RotatorFromAxisAndAngle` (0.0 1.0 0.0) (* (`KismetMathLibrary.Dot_VectorVector` (`KismetMathLibrary.Normal` _output_get_2) (1.0 1.0 1.0)) -45.0)) false false)
    (else
      (`SceneComponent.K2_SetRelativeRotation` _springarm (`KismetMathLibrary.RotatorFromAxisAndAngle` (0.0 0.0 1.0) (* (`KismetMathLibrary.Dot_VectorVector` (`KismetMathLibrary.Normal` _output_get_2) (1.0 1.0 1.0)) 45.0)) false false))))

(fn `turnGravR`
  (bind _springarm (`self.SpringArm`))
  ;[1 1 1] Change Gravity
  ;;[1 1 1] Turn Camera and Ball
  (bind _output_get (set `self.GravityFloorOrCeiling` (not (`self.GravityFloorOrCeiling`))))
  (bind _output_get_2 (set `self.Gravity` (`KismetMathLibrary.RotateAngleAxis` (`self.Gravity`) 90.0 (1.0 0.0 0.0))))
  (`SceneComponent.K2_AddLocalRotation` (`self.Camera`) (struct :`Roll` -90.0) false false)
  (`SceneComponent.K2_AddLocalRotation` (`self.Ball`) (struct :`Roll` -90.0) false false)
  ;;[1 1 1] Turn Camera Arm
  (if _output_get
    (`SceneComponent.K2_SetRelativeRotation` _springarm (`KismetMathLibrary.RotatorFromAxisAndAngle` (0.0 1.0 0.0) (* (`KismetMathLibrary.Dot_VectorVector` (`KismetMathLibrary.Normal` _output_get_2) (1.0 1.0 1.0)) -45.0)) false false)
    (else
      (`SceneComponent.K2_SetRelativeRotation` _springarm (`KismetMathLibrary.RotatorFromAxisAndAngle` (0.0 0.0 1.0) (* (`KismetMathLibrary.Dot_VectorVector` (`KismetMathLibrary.Normal` _output_get_2) (1.0 1.0 1.0)) 45.0)) false false))))

(fn `UserConstructionScript`)