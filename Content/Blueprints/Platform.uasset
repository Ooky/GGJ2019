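; Multi-behavior platform actor whose Mode selects sinking, disappearing or back-and-forth movement.
; Hit sinks it over SinkTime in mode 0; other modes play an Alpha timeline that destroys it at zero.
; Tick shuttles modes 2 and 3 along world X or Y by Speed per frame, reversing only on exact endpoint matches.
; BeginPlay sets those endpoints from Offset and zeroes Alpha in every mode, despite its "Mode 4 Invisible" label.
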(event `self.ReceiveHit`
  (params (MyComp :type "PrimitiveComponent Object Reference") (Other :type "Actor Object Reference") (OtherComp :type "PrimitiveComponent Object Reference") (bSelfMoved :type Boolean) (HitLocation :type "Vector Structure") (HitNormal :type "Vector Structure") (NormalImpulse :type "Vector Structure") (Hit :type "HitResult Structure (by ref)"))
  (switch `int` (`self.Mode`)
    (:`Default`
      ;[1 1 1] Mode 1: Disappear
      (bind (_direction _visibility) (`Timeline|Timeline_1` :!label _label)
        (:`Update`
          (if (!= _visibility 0.0)
            (`MeshComponent.SetScalarParameterValueOnMaterials` (`self.platform`) "Alpha" _visibility)
            (else
              (`self.K2_DestroyActor`))))))
    (:`0`
      ;[1 1 1] Mode 0: Sink
      (`KismetSystemLibrary.MoveComponentTo` (`self.platform`) (`KismetMathLibrary.TransformLocation` (`KismetMathLibrary.MakeTransform` (0.0 0.0 -1000.0)) (`SceneComponent.K2_GetComponentLocation` (`self.platform`))) (struct) false true (`self.sinkTime`) true))
    (:`1`
      (goto _label))))

(event `self.ReceiveBeginPlay`
  ;[1 1 1] Mode 2/3: Moving Forward/Backward or Left/Right
  ;;[1 1 1] 2: Forward Backward
  (`|ExecutionSequence`
    (:`then_0`
      (if (== (`self.Mode`) 2)
        (bind _output_get (set `self.initLocation` (`SceneComponent.K2_GetComponentLocation` (`self.platform`))))
        (set `self.targetLocation` (`KismetMathLibrary.MakeVector` (+ (.x _output_get) (`self.offset`)) (.y _output_get) (.z _output_get)))
        (else
          ;;[1 1 1] 3: Left Right
          (if (== (`self.Mode`) 3)
            (bind _output_get_2 (set `self.initLocation` (`SceneComponent.K2_GetComponentLocation` (`self.platform`))))
            (set `self.targetLocation` (`KismetMathLibrary.MakeVector` (.x _output_get_2) (+ (.y _output_get_2) (`self.offset`)) (.z _output_get_2)))))))
    (:`then_1`
      ;[1 1 1] Mode 4 Invisible
      (`MeshComponent.SetScalarParameterValueOnMaterials` (`self.platform`) "Alpha" 0.0))))

(event `self.ReceiveTick`
  (params (DeltaSeconds :type "Float (single-precision)"))
  (bind _platform (`self.platform`))
  (bind _platform_2 (`self.platform`))
  (bind _platform_3 (`self.platform`))
  (bind _platform_4 (`self.platform`))
  (bind _y (.y (`SceneComponent.K2_GetComponentLocation` _platform_4)))
  (bind _y_2 (.y (`SceneComponent.K2_GetComponentLocation` _platform)))
  (bind _x (.x (`SceneComponent.K2_GetComponentLocation` _platform_2)))
  (bind _x_2 (.x (`SceneComponent.K2_GetComponentLocation` _platform_3)))
  ;[1 1 1] Mode 2/3: Moving Forward/Backward or Left/Right
  ;;[1 1 1] 2: Forward Backward
  (if (== (`self.Mode`) 2)
    (if (`self.reverse`)
      (if (== (.x (`self.initLocation`)) _x_2)
        (set `self.reverse` false)
        (else
          (`SceneComponent.K2_SetWorldLocation` _platform_3 (`KismetMathLibrary.MakeVector` (- _x_2 (`self.speed`)) (.y (`SceneComponent.K2_GetComponentLocation` _platform_3)) (.z (`SceneComponent.K2_GetComponentLocation` _platform_3))) false false)))
      (elif (== (.x (`self.targetLocation`)) _x)
        (set `self.reverse` true)
        (else
          (`SceneComponent.K2_SetWorldLocation` _platform_2 (`KismetMathLibrary.MakeVector` (+ _x (`self.speed`)) (.y (`SceneComponent.K2_GetComponentLocation` _platform_2)) (.z (`SceneComponent.K2_GetComponentLocation` _platform_2))) false false))))
    (else
      ;;[1 1 1] 3: Left Right
      (if (== (`self.Mode`) 3)
        (if (`self.reverse`)
          (if (== (.y (`self.initLocation`)) _y_2)
            (set `self.reverse` false)
            (else
              (`SceneComponent.K2_SetWorldLocation` _platform (`KismetMathLibrary.MakeVector` (.x (`SceneComponent.K2_GetComponentLocation` _platform)) (- _y_2 (`self.speed`)) (.z (`SceneComponent.K2_GetComponentLocation` _platform))) false false)))
          (elif (== (.y (`self.targetLocation`)) _y)
            (set `self.reverse` true)
            (else
              (`SceneComponent.K2_SetWorldLocation` _platform_4 (`KismetMathLibrary.MakeVector` (.x (`SceneComponent.K2_GetComponentLocation` _platform_4)) (+ _y (`self.speed`)) (.z (`SceneComponent.K2_GetComponentLocation` _platform_4))) false false))))))))

(fn `UserConstructionScript`)