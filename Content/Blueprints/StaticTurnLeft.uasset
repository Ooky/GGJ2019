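; StaticTurnLeft is a trigger actor that rotates the player's gravity when its Right component is overlapped.
; Overlaps alternate between TurnGravL and TurnGravR on player pawn 0 via the TurnLeft flag, without checking which actor entered.
; A DoOnce blocks retriggering until 0.2 seconds after an overlap ends.
; Debug text names the opposite direction to the function called, and the construction script applies CubeColor to the Cube.
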(event `self.Right.OnComponentBeginOverlap`
  (params (OverlappedComponent :type "PrimitiveComponent Object Reference") (OtherActor :type "Actor Object Reference") (OtherComp :type "PrimitiveComponent Object Reference") (OtherBodyIndex :type Integer) (bFromSweep :type Boolean) (SweepResult :type "HitResult Structure (by ref)"))
  (bind _returnvalue (`GameplayStatics.GetPlayerPawn` 0))
  (bind _returnvalue_2 (`SceneComponent.K2_GetComponentLocation` (`Actor.RootComponent` (`GameplayStatics.GetPlayerPawn` 0))))
  (`/Engine/EditorBlueprintResources/StandardMacros.DoOnce` false :!label _label
    (:`Completed`
      (if (`self.turnLeft`)
        (bind _asplayer (cast `/Game/Blueprints/Player` _returnvalue))
        (`/Game/Blueprints/Player.turnGravL` _asplayer)
        (set `self.turnLeft` false)
        (`KismetSystemLibrary.DrawDebugString` _returnvalue_2 "Turned Right!" null (struct :`G` 1.0 :`B` 0.545189 :`A` 1.0) 2.0)
        (else
          (bind _asplayer_2 (cast `/Game/Blueprints/Player` _returnvalue))
          (`/Game/Blueprints/Player.turnGravR` _asplayer_2)
          (set `self.turnLeft` true)
          (`KismetSystemLibrary.DrawDebugString` _returnvalue_2 "Turned Left" null (struct :`R` 1.0 :`B` 0.01834 :`A` 1.0) 2.0))))))

(event `self.Right.OnComponentEndOverlap`
  (params (OverlappedComponent :type "PrimitiveComponent Object Reference") (OtherActor :type "Actor Object Reference") (OtherComp :type "PrimitiveComponent Object Reference") (OtherBodyIndex :type Integer))
  (`KismetSystemLibrary.Delay` 0.2)
  (goto _label :!via `Reset`))

(fn `UserConstructionScript`
  (`PrimitiveComponent.SetMaterial` (`self.Cube`) 0 (`self.CubeColor`)))